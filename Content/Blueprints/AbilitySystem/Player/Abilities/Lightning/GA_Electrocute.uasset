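; GA_Electrocute is a channeled player lightning ability that shocks the target under the mouse and chains to additional targets.
; A montage event locks movement, adds looping ShockLoop beam cues and starts a timer that commits cost and applies set-by-caller damage each tick.
; Input release (after a minimum spell time), failed cost or primary target death clears timer and cues, restores movement and commits cooldown.
; Additional targets that die drop out individually.
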(event Custom|DamageAndCost
  (bind _returnvalue (Ability|CommitAbilityCost false))
  (if _returnvalue
    (CallFunction|ApplyDamage)
    (else
      (CallFunction|ClearFunctionandEndABility))))

(event Ability|EventActivateAbility
  (CallFunction|EnforceImplementsCombatInterface)
  ;[0.001466 0.6649 1] Store Data
  (bind _datahandle (|TargetDataUnderMouse)
    (:ValidData
      (Class|RPGBeamSpell|StoreMouseDataInfo (Ability|TargetData|GetHitResultfromTargetData _datahandle))
      (Class|RPGBeamSpell|StoreOwnerVariables)
      (Utilities|FlowControl|Sequence
        (:then_0
          (Variables|/Script/Engine.PlayerController|SetbShowMouseCursor (Variables|Default|GetOwningPlayerController) false)
          (CallFunction|UpdateFacingTarget)
          (GameplayCue|ExecuteGameplayCue :GameplayCueTag "(TagName=\"GameplayCue.ShockBurst\")")
          (|PlayMontageandWaitProxy "None" (Variables|Default|GetMontage_Electrocute) 1.0 "None" false 1.0 0.0 false
            (:then
              (Ability|Tasks|WaitGameplayEvent "(TagName=\"Event.Montage.Electrocute\")" 0 true
                (:EventReceived
                  (CallFunction|InShockLoop)
                  (CallFunction|SpawnElectricBeam)
                  (bind _returnvalue (Utilities|Time|SetTimerbyEvent (delegate Custom|DamageAndCost) (Variables|Default|GetDamageDeltaTime) true))
                  (Variables|Default|SetDamageAndCostTimer _returnvalue))))))
        (:then_1
          ;[1 1 1] Enforce minimum spell time
          (bind _timeheld (Ability|Tasks|WaitInputRelease false)
            (:OnRelease
              (bind _output_get (Variables|Default|SetTime%20Held _timeheld))
              (if (< _output_get (Variables|Default|GetMinSpellTime))
                (Utilities|FlowControl|Delay (- (Variables|Default|GetMinSpellTime) (Variables|Default|GetTime%20Held))))
              (CallFunction|ClearFunctionandEndABility))))))))

(event EventPrimaryTargetDied
  (params (DeadActor :type Actor%20Object%20Reference))
  ;[1 1 1] Primary target died, we are done
  (GameplayCue|RemoveGameplayCueOnActor(Looping) DeadActor "(TagName=\"GameplayCue.ShockLoop\")" (Variables|Default|GetFirstTargetCueParams))
  (CallFunction|ClearFunctionandEndABility))

(event EventAdditionalTargetDied
  (params (DeadActor :type Actor%20Object%20Reference))
  ;[1 1 1] Additional target died, remove from map and shock loop cue
  (CallFunction|RemoveShockLoopCuefromAddtionalTarget DeadActor)
  (Utilities|Array|RemoveItem (Variables|Default|GetAdditional%20Targets) DeadActor))

(fn EnforceImplementsCombatInterface
  (if (not (Utilities|DoesObjectImplementInterface (Ability|GetAvatarActorfromActorInfo) "/Script/TopDownRPG.CombatInterface"))
    (Ability|EndAbility)))

(fn PreparetoEndAbility
  (Variables|/Script/Engine.PlayerController|SetbShowMouseCursor (Variables|Default|GetOwningPlayerController) true)
  (Class|CombatInterface|SetinShockLoop(Message) (Ability|GetAvatarActorfromActorInfo) false)
  (Pawn|Components|CharacterMovement|SetMovementMode (Variables|/Script/Engine.Character|GetCharacterMovement (Variables|Default|GetOwningCharacter)) "MOVE_Walking" 0)
  (if (Variables|Default|GetFirstTargetImplementsInterface)
    (GameplayCue|RemoveGameplayCueOnActor(Looping) (Variables|Default|GetMouseHitActor) "(TagName=\"GameplayCue.ShockLoop\")" (Variables|Default|GetFirstTargetCueParams))
    (for _array_element (Variables|Default|GetAdditional%20Targets)
      (CallFunction|RemoveShockLoopCuefromAddtionalTarget _array_element))
    (else
      (GameplayCue|RemoveGameplayCueOnActor(Looping) (Ability|GetAvatarActorfromActorInfo) "(TagName=\"GameplayCue.ShockLoop\")" (Variables|Default|GetFirstTargetCueParams)))))

(fn InShockLoop
  (Class|CombatInterface|SetinShockLoop(Message) (Ability|GetAvatarActorfromActorInfo) true)
  (Pawn|Components|CharacterMovement|DisableMovement (Variables|/Script/Engine.Character|GetCharacterMovement (Variables|Default|GetOwningCharacter))))

(fn UpdateFacingTarget
  (Class|CombatInterface|UpdateFacingTarget(Message) (Ability|GetAvatarActorfromActorInfo) (Variables|Default|GetMouseHitLocation)))

(fn SpawnElectricBeam
  (Class|RPGBeamSpell|TraceFirstTarget (Variables|Default|GetMouseHitLocation))
  (bind _returnvalue (Class|CombatInterface|GetWeapon(Message) (Variables|Default|GetOwningCharacter)))
  (Variables|Default|SetFirstTargetCueParams (Ability|GameplayCue|MakeGameplayCueParameters :Location (Variables|Default|GetMouseHitLocation) :SourceObject (Variables|Default|GetMouseHitActor) :TargetAttachComponent _returnvalue))
  (bind _output_get (Variables|Default|SetFirstTargetImplementsInterface (Utilities|DoesObjectImplementInterface (Variables|Default|GetMouseHitActor) "/Script/TopDownRPG.CombatInterface")))
  (if _output_get
    (Variables|Default|SetCueTarget (Variables|Default|GetMouseHitActor))
    (else
      (Variables|Default|SetCueTarget (Ability|GetAvatarActorfromActorInfo))))
  (GameplayCue|AddGameplayCueOnActor(Looping) (Variables|Default|GetCueTarget) "(TagName=\"GameplayCue.ShockLoop\")" (Variables|Default|GetFirstTargetCueParams))
  (if (Variables|Default|GetFirstTargetImplementsInterface)
    (bind _outadditionaltargets (Class|RPGBeamSpell|StoreAdditionalTargets))
    (bind _output_get_2 (Variables|Default|SetAdditional%20Targets _outadditionaltargets))
    (for _array_element _output_get_2
      (CallFunction|AddShockLoopCueToadditionaltarget _array_element))))

(fn AddShockLoopCueToadditionaltarget
  (params (AdditionalTarget :type Actor%20Object%20Reference))
  (LocalVariables|SetTargetActor AdditionalTarget)
  (Utilities|Map|Add (Variables|Default|GetAdditionalActorsToCUeParams) (LocalVariables|GetTargetActor) (Ability|GameplayCue|MakeGameplayCueParameters :Location (Transformation|GetActorLocation (LocalVariables|GetTargetActor)) :SourceObject (LocalVariables|GetTargetActor) :TargetAttachComponent (Variables|/Script/Engine.Actor|GetRootComponent (Variables|Default|GetMouseHitActor))))
  (GameplayCue|AddGameplayCueOnActor(Looping) (LocalVariables|GetTargetActor) "(TagName=\"GameplayCue.ShockLoop\")" (Ability|GameplayCue|MakeGameplayCueParameters :Location (Transformation|GetActorLocation (LocalVariables|GetTargetActor)) :SourceObject (LocalVariables|GetTargetActor) :TargetAttachComponent (Variables|/Script/Engine.Actor|GetRootComponent (Variables|Default|GetMouseHitActor)))))

(fn RemoveShockLoopCuefromAddtionalTarget
  (params (AdditionalTarget :type Actor%20Object%20Reference))
  (bind _additionalactorstocueparams (Variables|Default|GetAdditionalActorsToCUeParams))
  (bind (_value _returnvalue) (Utilities|Map|Find _additionalactorstocueparams AdditionalTarget))
  (if _returnvalue
    (GameplayCue|RemoveGameplayCueOnActor(Looping) AdditionalTarget "(TagName=\"GameplayCue.ShockLoop\")" _value)))

(fn ApplyDamage
  (CallFunction|ApplyDamageSingleTarget (Variables|Default|GetMouseHitActor))
  (for _array_element (Variables|Default|GetAdditional%20Targets)
    (CallFunction|ApplyDamageSingleTarget _array_element)))

(fn ApplyDamageSingleTarget
  (params (Actor :type Actor%20Object%20Reference))
  (bind _output_get (LocalVariables|SetDamageTarget Actor))
  (Utilities|IsValid _output_get
    (:Is%20Valid
      (bind _output_get_2 (LocalVariables|SetASC (Ability|GetAbilitySystemComponentfromActorInfo)))
      (Utilities|IsValid _output_get_2
        (:Is%20Valid
          (bind _returnvalue (Ability|GameplayEffect|AssignTagSetbyCallerMagnitude (GameplayEffects|MakeOutgoingSpec (LocalVariables|GetASC) (Variables|Default|GetDamageEffectClass) (Math|Conversions|ToFloat(Integer) (Ability|GetAbilityLevel)) (GameplayEffects|MakeEffectContext (LocalVariables|GetASC))) "(TagName=\"Damage.Lighting\")" (Class|RPGDamageGameplayAbility|GetDamageatLevel)))
          (Utilities|IsValid (Ability|GetAbilitySystemComponent (LocalVariables|GetDamageTarget))
            (:Is%20Valid
              (GameplayEffects|ApplyGameplayEffectSpecToSelf (Ability|GetAbilitySystemComponent (LocalVariables|GetDamageTarget)) _returnvalue))))))))

(fn ClearFunctionandEndABility
  (Utilities|Time|ClearandInvalidateTimerbyHandle (Variables|Default|GetDamageAndCostTimer))
  (CallFunction|PreparetoEndAbility)
  (Ability|CommitAbilityCooldown false)
  (Utilities|Array|Clear (Variables|Default|GetAdditional%20Targets))
  (Utilities|Map|Clear (Variables|Default|GetAdditionalActorsToCUeParams))
  (Variables|Default|SetMouseHitActor 0)
  (Variables|Default|SetFirstTargetImplementsInterface false)
  (Variables|Default|SetTime%20Held 0.0)
  (Ability|EndAbility))