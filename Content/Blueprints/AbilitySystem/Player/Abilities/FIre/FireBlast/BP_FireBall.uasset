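; BP_FireBall is the fireball actor for the player's FireBlast ability, flying outward and then homing back to ReturnToActor like a boomerang.
; StartOutGoingTimeline runs on the authority only, using a timeline to lerp it forward by TravelDIstance.
; A second timeline then lerps it from that apex toward the target's live location.
; Once within ExplodeDistance on the return, it calls OnHit and destroys itself.
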(event EventBeginPlay)

(event Collision|EventActorBeginOverlap
  (params (OtherActor :type Actor%20Object%20Reference)))

(event EventTick
  (params (DeltaSeconds :type Float%20%28single-precision%29)))

(event EventStartOutGoingTimeline
  ;[1 0.7595 0] Store Intial and Apex Location
  (Networking|SwitchHasAuthority
    (:Authority
      (Variables|Default|SetIntialLocation (Transformation|GetActorLocation))
      (Variables|Default|SetApexLocation (+ (Variables|Default|GetIntialLocation) (* (Transformation|GetActorForwardVector) (Variables|Default|GetTravel%20DIstance))))
      (bind _outgointrack (Timeline|OutGoingTimeline Play)
        (:Update
          (Transformation|SetActorLocation (Math|Vector|Lerp(Vector) (Variables|Default|GetIntialLocation) (Variables|Default|GetApexLocation) _outgointrack) false false))
        (:Finished
          (bind _returningtrack (Timeline|ReturningTimeline Play)
            (:Update
              (Transformation|SetActorLocation (Math|Vector|Lerp(Vector) (Variables|Default|GetApexLocation) (Transformation|GetActorLocation (Variables|Default|GetReturnToActor)) _returningtrack) false false)
              (if (CallFunction|IsWithinExplodeDistance)
                (Class|RPGProjectile|OnHit)
                (Actor|DestroyActor)))))))))

(fn ConstructionScript)

(fn IsWithinExplodeDistance
  (return (<= (Math|Vector|VectorLength (- (Transformation|GetActorLocation) (Transformation|GetActorLocation (Variables|Default|GetReturnToActor)))) (Variables|Default|GetExplodeDistance))))