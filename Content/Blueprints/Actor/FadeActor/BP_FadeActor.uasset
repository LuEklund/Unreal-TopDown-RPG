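; BP_FadeActor is an actor that fades its mesh out and in, doing both on BeginPlay one second apart.
; The construction script caches original materials and builds dynamic instances from fade materials.
; FadeOut swaps those in and plays a timeline driving their "Fade" parameter; FadeIn reverses it.
; When the timeline finishes, a value of 1 restores the originals and blocks Visibility traces, while 0 ignores them.
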(event Custom|FadeOut
  (CallFunction|SetMaterialstoDynamicInstances)
  (bind _fade (Timeline|FadeTimeLine Play)
    (:Update
      (for _array_element (Variables|Default|GetDynamicMaterialInstances)
        (Rendering|Material|SetScalarParameterValue _array_element "Fade" _fade :!class /Script/Engine.MaterialInstanceDynamic)))
    (:Finished
      (CallFunction|FadeFinnished _fade))))

(event Custom|FadeIn
  (bind _fade (Timeline|FadeTimeLine Reverse)
    (:Update
      (for _array_element (Variables|Default|GetDynamicMaterialInstances)
        (Rendering|Material|SetScalarParameterValue _array_element "Fade" _fade :!class /Script/Engine.MaterialInstanceDynamic)))
    (:Finished
      (CallFunction|FadeFinnished _fade))))

(event EventBeginPlay
  (CallFunction|FadeOut)
  (Utilities|FlowControl|Delay 1.0)
  (CallFunction|Fadein))

(fn ConstructionScript
  (Utilities|Array|Clear (Variables|Default|GetDynamicMaterialInstances))
  (Variables|Default|SetOriginal%20Materials (Rendering|Material|GetMaterials (Variables|Default|GetMesh)))
  (for _array_element (Variables|Default|GetFadeMaterialInstances)
    (bind _returnvalue (Rendering|Material|CreateDynamicMaterialInstance _array_element "None" "None" :!class /Script/Engine.KismetMaterialLibrary))
    (Utilities|Array|AddUnique (Variables|Default|GetDynamicMaterialInstances) _returnvalue)))

(fn SetMaterialstoDynamicInstances
  (for (_array_element _array_index) (Variables|Default|GetDynamicMaterialInstances)
    (Rendering|Material|SetMaterial (Variables|Default|GetMesh) _array_index _array_element)))

(fn ResetMaterials
  (for (_array_element _array_index) (Variables|Default|GetOriginal%20Materials)
    (Rendering|Material|SetMaterial (Variables|Default|GetMesh) _array_index _array_element)))

(fn FadeFinnished
  (params (A :type Float%20%28double-precision%29))
  (if (>= A 1.0)
    (CallFunction|ResetMaterials)
    (Collision|SetCollisionResponsetoChannel (Variables|Default|GetMesh) "ECC_Visibility" "ECR_Block")
    (elif (<= A 0.0)
      (Collision|SetCollisionResponsetoChannel (Variables|Default|GetMesh) "ECC_Visibility" "ECR_Ignore"))))