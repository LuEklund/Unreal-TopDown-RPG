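; BP_FlamePillar is a flame pillar actor whose point light flickers continuously during play.
; BeginPlay randomly picks one of two FlameIntensity timelines to play from the start, and each picks again when it finishes, forming an endless varied loop.
; Each timeline update feeds ScaleFlameInensity, which sets the PointLight intensity to the curve value multiplied by BaseIntensity.
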(event Custom|StartTimeLine_1
  (bind _flameintensity (Timeline|FlameIntensity_1 PlayFromStart)
    (:Update
      (CallFunction|ScaleFlameInensity _flameintensity))
    (:Finished
      (CallFunction|ChooseTimeline))))

(event Custom|StartTimeLine_2
  (bind _flameintensity (Timeline|FlameIntensity_2 PlayFromStart)
    (:Update
      (CallFunction|ScaleFlameInensity _flameintensity))
    (:Finished
      (CallFunction|ChooseTimeline))))

(event Custom|Choose%20Timeline
  (switch int (Math|Random|RandomIntegerinRange 0 1)
    (:Default
      (CallFunction|StartTimeLine2 :!label _label))
    (:0
      (CallFunction|StartTimeLine1))
    (:1
      (goto _label))))

(event EventBeginPlay
  (CallFunction|ChooseTimeline))

(fn ConstructionScript)

(fn ScaleFlameInensity
  (params (Flame%20Intensity :type Float%20%28double-precision%29))
  (Rendering|Components|Light|SetIntensity (Variables|Default|GetPointLight) (* Flame%20Intensity (Variables|Default|GetBaseIntensity))))